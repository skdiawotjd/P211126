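; Player-controlled airplane pawn with two spinning propellers and a single launchable rocket.
; Axis inputs steer the view and move it along the control yaw's horizontal plane, while a looping timer rotates the propellers by Speed.
; Key 1 triggers Fire via timer, enabling rocket physics, pushing it by the body's forward vector scaled mainly on world X, and playing audio.
; On hit, the rocket stops the audio, spawns explosion effects and destroys itself.
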(event OnComponentHit(SM_Rocket)
  (params (HitComponent :type Primitive%20Component%20Object%20Reference) (OtherActor :type Actor%20Object%20Reference) (OtherComp :type Primitive%20Component%20Object%20Reference) (NormalImpulse :type Vector :default "0, 0, 0") (Hit :type Hit%20Result%20Structure%20%28by%20ref%29))
  (Audio|Components|Audio|Stop (Variables|Default|GetAudio))
  (Effects|SpawnEmitteratLocation "/Game/StarterContent/Particles/P_Explosion.P_Explosion" (Transformation|GetWorldLocation (Variables|Default|GetSM_Rocket)))
  (Audio|SpawnSoundatLocation "/Game/StarterContent/Audio/Explosion_Cue.Explosion_Cue" (Transformation|GetActorLocation OtherActor) "0, 0, 0" 0.1 1.0 0.0 0 0)
  (Components|DestroyComponent (Variables|Default|GetSM_Rocket)))

(event EventBeginPlay
  (Utilities|Time|SetTimerbyFunctionName 0 "RotatePropeller" 0.01 true))

(event Collision|EventActorBeginOverlap
  (params (OtherActor :type Actor%20Object%20Reference)))

(event EventTick
  (params (DeltaSeconds :type Float%20%28single-precision%29)))

(event Input|AxisEvents|InputAxisLookUp
  (params (AxisValue :type Float%20%28single-precision%29))
  (Pawn|Input|AddControllerPitchInput AxisValue))

(event Input|AxisEvents|InputAxisTurn
  (params (AxisValue :type Float%20%28single-precision%29))
  (Pawn|Input|AddControllerYawInput AxisValue))

(event Input|AxisEvents|InputAxisMoveForward
  (params (AxisValue :type Float%20%28single-precision%29))
  (Pawn|Input|AddMovementInput (Math|Vector|GetForwardVector (Math|Rotator|MakeRotator 0.0 0.0 (.Yaw (Math|Rotator|BreakRotator (Pawn|GetControlRotation :!class /Script/Engine.Pawn))))) AxisValue false))

(event Input|AxisEvents|InputAxisMoveRight
  (params (AxisValue :type Float%20%28single-precision%29))
  (Pawn|Input|AddMovementInput (Math|Vector|GetRightVector (Math|Rotator|MakeRotator 0.0 0.0 (.Yaw (Math|Rotator|BreakRotator (Pawn|GetControlRotation :!class /Script/Engine.Pawn))))) AxisValue false))

(event Input|KeyboardEvents|1
  (params (Key :type Key%20Structure :default "None"))
  (:Pressed
    (Utilities|Time|SetTimerbyFunctionName 0 "Fire" 0.01)))

(fn ConstructionScript)

(fn RotatePropeller
  (bind _speed (Variables|Default|GetSpeed))
  (bind _returnvalue (* 0.01 _speed))
  (Transformation|AddRelativeRotation (Variables|Default|GetSM_P38_Propeller1) (Math|Rotator|MakeRotator _returnvalue 0.0 0.0) false false)
  (Transformation|AddRelativeRotation (Variables|Default|GetSM_P38_Propeller2) (Math|Rotator|MakeRotator _returnvalue 0.0 0.0) false false))

(fn Fire
  (bind _sm_rocket (Variables|Default|GetSM_Rocket))
  (Physics|SetSimulatePhysics _sm_rocket true)
  (Collision|SetCollisionEnabled _sm_rocket "QueryAndPhysics")
  (Physics|AddForce _sm_rocket (* (Math|Vector|GetForwardVector (Variables|Default|GetSM_Body)) "1000000.000000,1.000000,1.000000") "None" false)
  (Audio|Components|Audio|Play (Variables|Default|GetAudio) 0.2))